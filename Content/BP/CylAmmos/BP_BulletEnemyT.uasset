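; BP_BulletEnemyT is an enemy bullet actor that spawns explosions on impact and destroys itself 20 seconds after BeginPlay.
; Its Box overlap spawns BP_Explosion at the bullet's transform for actors tagged "Collision" or actors that cast to BP_Pawn.
; Only the pawn branch then destroys the bullet after a short delay; after a "Collision" hit it stays until the lifetime expires.
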(event OnComponentBeginOverlap(Box)
  (params (OverlappedComponent :type Primitive%20Component%20Object%20Reference) (OtherActor :type Actor%20Object%20Reference) (OtherComp :type Primitive%20Component%20Object%20Reference) (OtherBodyIndex :type Integer) (bFromSweep :type Boolean) (SweepResult :type Hit%20Result%20Structure%20%28by%20ref%29))
  (if (Actor|ActorHasTag OtherActor "Collision")
    (Game|SpawnActorfromClass "/Game/BP/CylAmmos/BP_Explosion.BP_Explosion_C" (Transformation|GetActorTransform) "Undefined" 0 0)
    (else
      (Utilities|Casting|CastToBP_Pawn OtherActor)
      (Game|SpawnActorfromClass "/Game/BP/CylAmmos/BP_Explosion.BP_Explosion_C" (Transformation|GetActorTransform) "Undefined" 0 0)
      (Utilities|FlowControl|Delay 0.1)
      (Actor|DestroyActor))))

(event EventBeginPlay
  (Utilities|FlowControl|Delay 2e+01)
  (Actor|DestroyActor))

(fn ConstructionScript)